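; BP_BulletEnemy is an enemy bullet that damages the player's hero on hit.
; On BeginPlay it caches the player character as a BP_HeroChar and, if that cast succeeds, sets a two-second lifespan.
; Any hit destroys the bullet, and a hit on the cached hero first calls HeroDamage with its Damage value.
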(event `self.ReceiveBeginPlay`
  (bind _asbp_hero_char (cast `/Game/HeroChar/BP_HeroChar` (`GameplayStatics.GetPlayerCharacter` 0)))
  (set `self.HeroCharRefer` _asbp_hero_char)
  (`self.SetLifeSpan` 2.0))

(event `self.ReceiveHit`
  (params (MyComp :type "PrimitiveComponent Object Reference") (Other :type "Actor Object Reference") (OtherComp :type "PrimitiveComponent Object Reference") (bSelfMoved :type Boolean) (HitLocation :type "Vector Structure") (HitNormal :type "Vector Structure") (NormalImpulse :type "Vector Structure") (Hit :type "HitResult Structure (by ref)"))
  (if (== Other (`self.HeroCharRefer`))
    (`/Game/HeroChar/BP_HeroChar.HeroDamage` (`self.HeroCharRefer`) (`self.Damage`))
    (`self.K2_DestroyActor`)
    (else
      (`self.K2_DestroyActor`))))

(fn `UserConstructionScript`)