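; Enemy actor that turns to face the hero and repeatedly fires BP_BulletEnemy from its Arrow once alerted.
; Any capsule overlap or a Hit alerts it, after which Tick tracks the hero and starts a looping Fire timer once, which StopEnemy clears.
; Hit also subtracts health and destroys the actor at zero.
; A randomized-rate timeline is set up for vertical bobbing, but the graph never starts it.
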(event `self.ReceiveBeginPlay`
  (bind _returnvalue (`self.K2_GetActorLocation`))
  (`|ExecutionSequence`
    (:`then_0`
      ;[1 1 1] Set Start End Location / Set Timeline Play Rate
      (set `self.StartLocation` _returnvalue)
      (set `self.EndLocation` (+ _returnvalue (`KismetMathLibrary.MakeVector` 0.0 0.0 (`KismetMathLibrary.RandomFloatInRange` 50.0 100.0))))
      (`TimelineComponent.SetPlayRate` (`self.EnemyLoop`) (`KismetMathLibrary.RandomFloatInRange` 1.0 2.0)))
    (:`then_1`
      ;[1 1 1] Get Hero Char Refer
      (bind _asbp_hero_char (cast `/Game/HeroChar/BP_HeroChar` (`GameplayStatics.GetPlayerCharacter` 0)))
      (set `self.HeroCharRefer` _asbp_hero_char))))

(event `self.ReceiveTick`
  (params (DeltaSeconds :type "Float (single-precision)"))
  ;[1 1 1] Set Actor Rotation when see Hero
  (if (or (`self.isHeroOnSight`) (`self.isHeroHere`))
    (`|ExecutionSequence`
      (:`then_0`
        (`self.K2_SetActorRotation` (`KismetMathLibrary.FindLookAtRotation` (`self.K2_GetActorLocation`) (`self.K2_GetActorLocation` (`self.HeroCharRefer`)))))
      (:`then_1`
        (`/Engine/EditorBlueprintResources/StandardMacros.DoOnce` false
          (:`Completed`
            (`KismetSystemLibrary.K2_SetTimer` null "Fire" (/ 1.0 (`self.ShootPerSeconds`)) true)))))))

(event `self.Capsule.OnComponentBeginOverlap`
  (params (OverlappedComponent :type "PrimitiveComponent Object Reference") (OtherActor :type "Actor Object Reference") (OtherComp :type "PrimitiveComponent Object Reference") (OtherBodyIndex :type Integer) (bFromSweep :type Boolean) (SweepResult :type "HitResult Structure (by ref)"))
  ;[1 1 1] Overlap - Set HeroOnSight
  (set `self.isHeroOnSight` true))

(event `StopEnemy`
  ;[1 1 1] Stop Enemy
  (`KismetSystemLibrary.K2_ClearTimer` null "Fire"))

(event `self.ReceiveHit`
  (params (MyComp :type "PrimitiveComponent Object Reference") (Other :type "Actor Object Reference") (OtherComp :type "PrimitiveComponent Object Reference") (bSelfMoved :type Boolean) (HitLocation :type "Vector Structure") (HitNormal :type "Vector Structure") (NormalImpulse :type "Vector Structure") (Hit :type "HitResult Structure (by ref)"))
  ;[1 1 1] Hit
  (set `self.isHeroHere` true)
  (bind _output_get (set `self.EnemyHealth` (- (`self.EnemyHealth`) (`self.Damage`))))
  (`KismetSystemLibrary.PrintString` (`KismetStringLibrary.Conv_DoubleToString` _output_get))
  (if (<= (`self.EnemyHealth`) 0.0)
    (`KismetSystemLibrary.PrintString` "Enemy is Dead")
    (`self.K2_DestroyActor`)))

(fn `Fire`
  (`|SpawnActorFromClass` "/Game/Enemy/BP_BulletEnemy.BP_BulletEnemy_C" (`SceneComponent.K2_GetComponentToWorld` (`self.Arrow`)) "Undefined" "OverrideRootScale" null null))

(fn `UserConstructionScript`)