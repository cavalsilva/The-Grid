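; Gun Blueprint with trigger events that start and stop firing.
; ActiveTrigger fires immediately, then sets a function-name timer, with no looping flag shown, to call Fire again after an interval derived from ShootPerSeconds.
; DesactiveTrigger clears that timer.
; Fire spawns an actor at the ArrowBullet component's transform, with no class specified here, and prints a debug message.
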(event `ActiveTrigger`
  ;[1 1 1] Active Trigger / Desactive Trigger / Fire
  (`self.Fire`)
  (`KismetSystemLibrary.K2_SetTimer` null "Fire" (/ 1.0 (`self.ShootPerSeconds`))))

(event `DesactiveTrigger`
  ;[1 1 1] Active Trigger / Desactive Trigger / Fire
  (`KismetSystemLibrary.K2_ClearTimer` null "Fire"))

(fn `Fire`
  (`|SpawnActorFromClass` "/Game/HeroChar/Gun/SK_Gun/BP_Bullet.BP_Bullet_C" (`SceneComponent.K2_GetComponentToWorld` (`self.ArrowBullet`)) "Undefined" "OverrideRootScale" null null)
  (`KismetSystemLibrary.PrintString` "Fire"))

(fn `UserConstructionScript`)