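; BP_Totem is a colored totem (pink, green or blue) that activates on Interact if the game mode reports the matching key picked.
; Activation plays a timeline raising the hoop, brightens the glow material set in construction, increments the active-totem count and triggers the all-active check.
; Interact also spawns a BP_KeyFixed tinted with glowing dynamic materials, regardless of the key check, with no repeat guard.
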(event `self.ReceiveBeginPlay`
  (bind _asbp_gameplay_game_mode (cast `/Game/GameLogic/BP_GamePlayGameMode` (`GameplayStatics.GetGameMode`)))
  (set `self.GameModeRefer` _asbp_gameplay_game_mode))

(event `/Game/Objects/Totem/BI_Interactable.Interact`
  ;[1 1 1] Blueprint Interface Interact - Active Totem - Spawn Key - Create Material
  (switch `/Game/Objects/Key/EKeys` (`self.TotemType`)
    (:`NewEnumerator0`
      (`self.ActiveTotemPink`)
      (bind _returnvalue (`self.SpawnKey`))
      (`self.CreateKeyMaterial` (`/Game/Objects/Key/BP_KeyFixed.Frame1` _returnvalue) (`/Game/Objects/Key/BP_KeyFixed.Frame2` _returnvalue) (`self.PinkColor`)))
    (:`NewEnumerator1`
      (`self.ActiveTotemGreen`)
      (bind _returnvalue_2 (`self.SpawnKey`))
      (`self.CreateKeyMaterial` (`/Game/Objects/Key/BP_KeyFixed.Frame1` _returnvalue_2) (`/Game/Objects/Key/BP_KeyFixed.Frame2` _returnvalue_2) (`self.GreenColor`)))
    (:`NewEnumerator2`
      (`self.ActiveTotemBlue`)
      (bind _returnvalue_3 (`self.SpawnKey`))
      (`self.CreateKeyMaterial` (`/Game/Objects/Key/BP_KeyFixed.Frame1` _returnvalue_3) (`/Game/Objects/Key/BP_KeyFixed.Frame2` _returnvalue_3) (`self.BlueColor`)))))

(event `ActiveTotemPink`
  (bind _gamemoderefer (`self.GameModeRefer`))
  ;[1 1 1] Active Totems - Check isPickKey - Play Totem Animation
  (if (`/Game/GameLogic/BP_GamePlayGameMode.isPickKeyPink` (`self.GameModeRefer`))
    (`TimelineComponent.PlayFromStart` (`self.TotemAnimation`))
    (`MaterialInstanceDynamic.SetScalarParameterValue` (`self.TotemMaterial`) "Emissive" (`self.EmissiveIntensityActive`))
    (`/Game/GameLogic/BP_GamePlayGameMode.IncrementNumberOfTotemsActive` _gamemoderefer)
    (`/Game/GameLogic/BP_GamePlayGameMode.CheckAllTotemsActive` _gamemoderefer)))

(event `ActiveTotemGreen`
  (bind _gamemoderefer (`self.GameModeRefer`))
  ;[1 1 1] Active Totems - Check isPickKey - Play Totem Animation
  (if (`/Game/GameLogic/BP_GamePlayGameMode.isPickKeyGreen` (`self.GameModeRefer`))
    (`TimelineComponent.PlayFromStart` (`self.TotemAnimation`))
    (`MaterialInstanceDynamic.SetScalarParameterValue` (`self.TotemMaterial`) "Emissive" (`self.EmissiveIntensityActive`))
    (`/Game/GameLogic/BP_GamePlayGameMode.IncrementNumberOfTotemsActive` _gamemoderefer)
    (`/Game/GameLogic/BP_GamePlayGameMode.CheckAllTotemsActive` _gamemoderefer)))

(event `ActiveTotemBlue`
  (bind _gamemoderefer (`self.GameModeRefer`))
  ;[1 1 1] Active Totems - Check isPickKey - Play Totem Animation
  (if (`/Game/GameLogic/BP_GamePlayGameMode.isPickKeyBlue` (`self.GameModeRefer`))
    (`TimelineComponent.PlayFromStart` (`self.TotemAnimation`))
    (`MaterialInstanceDynamic.SetScalarParameterValue` (`self.TotemMaterial`) "Emissive" (`self.EmissiveIntensityActive`))
    (`/Game/GameLogic/BP_GamePlayGameMode.IncrementNumberOfTotemsActive` _gamemoderefer)
    (`/Game/GameLogic/BP_GamePlayGameMode.CheckAllTotemsActive` _gamemoderefer)))

(fn `CreateKeyMaterial`
  (params (Target1 :type "PrimitiveComponent Object Reference") (Target2 :type "PrimitiveComponent Object Reference") (ColorMaterial :type "LinearColor Structure"))
  (bind _returnvalue (`PrimitiveComponent.CreateDynamicMaterialInstance` Target1 1 "/Game/Materials/M_Glow.M_Glow"))
  (`MaterialInstanceDynamic.SetVectorParameterValue` _returnvalue "BaseColor" ColorMaterial)
  (`MaterialInstanceDynamic.SetScalarParameterValue` _returnvalue "Emissive" 20.0)
  (bind _returnvalue_2 (`PrimitiveComponent.CreateDynamicMaterialInstance` Target2 1 "/Game/Materials/M_Glow.M_Glow"))
  (`MaterialInstanceDynamic.SetVectorParameterValue` _returnvalue_2 "BaseColor" ColorMaterial)
  (`MaterialInstanceDynamic.SetScalarParameterValue` _returnvalue_2 "Emissive" 20.0))

(fn `SpawnKey`
  (returns (ReturnValue :type "/Game/Objects/Key/BP_KeyFixed Object Reference"))
  (bind _returnvalue (`|SpawnActorFromClass` "/Game/Objects/Key/BP_KeyFixed.BP_KeyFixed_C" (`SceneComponent.K2_GetComponentToWorld` (`self.KeySpawnTransform`)) "Undefined" "OverrideRootScale" null null))
  (return _returnvalue))

(fn `UserConstructionScript`
  (bind _returnvalue (`PrimitiveComponent.CreateDynamicMaterialInstance` (`self.TotemBase`) 1 "/Game/Materials/M_Glow.M_Glow"))
  (bind _output_get (set `self.TotemMaterial` _returnvalue))
  (`MaterialInstanceDynamic.SetScalarParameterValue` _output_get "Emissive" (`self.EmissiveIntensity`))
  (`MaterialInstanceDynamic.SetVectorParameterValue` _output_get "BaseColor" (`self.BaseColor`)))